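; Four-way junction piece for the spline road tool that spawns BP_SplineRoadGenerator actors at its connection sockets.
; The construction script shows or hides the sidewalk from ShowSideWalk.
; Two numbered events drive SpawnRoad, which places a generator at the chosen base-mesh socket's location and rotation.
; The single-road event uses the Socket variable, while the all-roads event fills Conn1, Conn3 and Conn4, leaving out Conn2.
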(event `01_SpawnSingleRoad`
  (`self.SpawnRoad` (`self.Socket`)))

(event `02_SpawnAllRoads`
  (`|ExecutionSequence`
    (:`then_0`
      (`self.SpawnRoad` "NewEnumerator0"))
    (:`then_1`
      (`self.SpawnRoad` "NewEnumerator2"))
    (:`then_2`
      (`self.SpawnRoad` "NewEnumerator3"))))

(fn `SpawnRoad`
  (params (Selection :type "/Game/SplineRoadTool/Blueprints/Data/ENUM_SocketNumber Enum" :default "NewEnumerator0"))
  (bind _basestaticmesh (`self.BaseStaticMesh`))
  (bind _basestaticmesh_2 (`self.BaseStaticMesh`))
  (bind _basestaticmesh_3 (`self.BaseStaticMesh`))
  (bind _basestaticmesh_4 (`self.BaseStaticMesh`))
  (switch `/Game/SplineRoadTool/Blueprints/Data/ENUM_SocketNumber` Selection
    (:`NewEnumerator0`
      ;[1 1 1] Conn1
      (`|SpawnActorFromClass` "/Game/SplineRoadTool/Blueprints/BP_SplineRoadGenerator.BP_SplineRoadGenerator_C" (`KismetMathLibrary.MakeTransform` (`SceneComponent.GetSocketLocation` _basestaticmesh_2 "Conn1") (`SceneComponent.GetSocketRotation` _basestaticmesh_2 "Conn1")) "AlwaysSpawn" "OverrideRootScale" null null))
    (:`NewEnumerator1`
      ;[1 1 1] Conn2
      (`|SpawnActorFromClass` "/Game/SplineRoadTool/Blueprints/BP_SplineRoadGenerator.BP_SplineRoadGenerator_C" (`KismetMathLibrary.MakeTransform` (`SceneComponent.GetSocketLocation` _basestaticmesh_3 "Conn2") (`SceneComponent.GetSocketRotation` _basestaticmesh_3 "Conn2")) "AlwaysSpawn" "OverrideRootScale" null null))
    (:`NewEnumerator2`
      ;[1 1 1] Conn3
      (`|SpawnActorFromClass` "/Game/SplineRoadTool/Blueprints/BP_SplineRoadGenerator.BP_SplineRoadGenerator_C" (`KismetMathLibrary.MakeTransform` (`SceneComponent.GetSocketLocation` _basestaticmesh "Conn3") (`SceneComponent.GetSocketRotation` _basestaticmesh "Conn3")) "AlwaysSpawn" "OverrideRootScale" null null))
    (:`NewEnumerator3`
      ;[1 1 1] Conn4
      (`|SpawnActorFromClass` "/Game/SplineRoadTool/Blueprints/BP_SplineRoadGenerator.BP_SplineRoadGenerator_C" (`KismetMathLibrary.MakeTransform` (`SceneComponent.GetSocketLocation` _basestaticmesh_4 "Conn4") (`SceneComponent.GetSocketRotation` _basestaticmesh_4 "Conn4")) "AlwaysSpawn" "OverrideRootScale" null null))))

(fn `UserConstructionScript`
  (`SceneComponent.SetVisibility` (`self.SideWalk`) (`self.showSideWalk`) false))