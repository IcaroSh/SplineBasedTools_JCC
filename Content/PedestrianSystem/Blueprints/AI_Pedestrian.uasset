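; AI controller that makes a pedestrian wander between point actors in the world, starting shortly after BeginPlay.
; NextPoint sphere-traces ahead for point objects, ignoring the current one, rotating through right, back, left and forward and widening the search when nothing is found.
; A random hit briefly flashes yellow, then the pawn moves near a randomly indexed hit location and repeats on arrival or failure.
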(event `self.ReceiveBeginPlay`
  (`KismetSystemLibrary.Delay` 2.0)
  (`self.NextPoint`))

(event `Go_to`
  (params (Target :type "Vector Structure"))
  (`|AIMoveTo` null Target null 100.0
    (:`OnSuccess`
      _)
    (:`OnFail`
      (`KismetSystemLibrary.Delay` 0.5)))
  (`self.NextPoint`))

(event `NextPoint`
  (bind _returnvalue (`self.K2_GetPawn`))
  (bind _returnvalue_2 (+ (* (`self.vectorTrackLocation`) (`self.Distance`)) (`self.K2_GetActorLocation` (`self.K2_GetPawn`))))
  (set `self.Distance` 3000.0)
  (set `self.vectorTrackLocation` (`self.GetActorForwardVector` (`self.K2_GetPawn`)))
  (bind (_outhits _returnvalue_3) (`KismetSystemLibrary.SphereTraceMultiForObjects` _returnvalue_2 (+ _returnvalue_2 (1.0 0.0 0.0)) (`self.Radius`) (`|MakeArray` "ObjectTypeQuery7" :!type "EObjectTypeQuery Enum") false (`|MakeArray` (`self.CurrentPoint`)) "ForDuration" :!label _label))
  (if _returnvalue_3
    (bind (_bblockinghit _binitialoverlap _time _distance _location _impactpoint _normal _impactnormal _physmat _hitactor) (`GameplayStatics.BreakHitResult` (`|GetArrayItem` _outhits (`KismetMathLibrary.RandomInteger` (`KismetArrayLibrary.Array_Length` _outhits)))))
    (bind _output_get (set `self.CurrentPoint` _hitactor))
    (`PrimitiveComponent.SetMaterial` (`self.GetComponentByClass` _output_get "/Script/Engine.StaticMeshComponent") 0 "/Game/PedestrianSystem/MI_Yellow.MI_Yellow")
    (`KismetSystemLibrary.Delay` 1.5)
    (`PrimitiveComponent.SetMaterial` (`self.GetComponentByClass` _output_get "/Script/Engine.StaticMeshComponent") 0 "/Game/PedestrianSystem/MI_Red.MI_Red")
    (`self.Go_to` (`NavigationSystemV1.K2_GetRandomReachablePointInRadius` _impactpoint 100.0 null null))
    (else
      (switch `int` (`self.NumberOfPasses`)
        (:`0`
          (set `self.vectorTrackLocation` (`self.GetActorRightVector` _returnvalue)))
        (:`1`
          (set `self.vectorTrackLocation` (* (`self.GetActorForwardVector` _returnvalue) -1.0)))
        (:`2`
          (set `self.vectorTrackLocation` (* (`self.GetActorRightVector` _returnvalue) -1.0)))
        (:`3`
          (set `self.vectorTrackLocation` (`self.GetActorForwardVector` _returnvalue)))
        (:`4`
          (set `self.Distance` (+ (`self.Distance`) 100.0))
          (set `self.Radius` (+ (`self.Radius`) 100.0))))
      (`/Engine/EditorBlueprintResources/StandardMacros.IncrementInt` (`self.NumberOfPasses`)
        (:`  `
          (if (> (`self.NumberOfPasses`) 4)
            (set `self.NumberOfPasses` 0))
          (`KismetSystemLibrary.Delay` 0.2)
          (goto _label))))))

(fn `UserConstructionScript`)