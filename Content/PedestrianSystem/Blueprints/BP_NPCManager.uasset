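; BP_NPCManager is a pedestrian spawner that keeps a target NPC count around itself while the player is within range.
; After a randomized startup delay, Tick triggers a DoOnce-guarded, delayed spawn loop that places NPCs at random reachable nearby points.
; It reuses NPCs from a GameState-held pool before spawning new BP_Pedestrians.
; Tick also hides NPCs too far from the player and returns them to that pool.
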(event `self.ReceiveBeginPlay`
  (`|ExecutionSequence`
    (:`then_0`
      (bind _returnvalue (`GameplayStatics.GetActorOfClass` "/Game/PedestrianSystem/ThirdPersonBP/Blueprints/ThirdPersonCharacter.ThirdPersonCharacter_C"))
      (set `self.PlayerRef` _returnvalue))
    (:`then_1`
      (`KismetSystemLibrary.Delay` (`KismetMathLibrary.RandomFloatInRange` 0.5 1.0))
      (`self.SetActorTickEnabled` true))))

(event `self.ReceiveTick`
  (params (DeltaSeconds :type "Float (single-precision)"))
  (`|ExecutionSequence`
    (:`then_0`
      (if (< (`KismetMathLibrary.Vector_Distance` (`self.K2_GetActorLocation` (`self.PlayerRef`)) (`self.K2_GetActorLocation`)) (`self.SpawnerRange`))
        (`self.SpawnNPC`)))
    (:`then_1`
      (`self.CheckNPCLocation`))))

(event `SpawnNPC`
  (bind _randomlocation (`NavigationSystemV1.K2_GetRandomReachablePointInRadius` (`self.K2_GetActorLocation`) 200.0 null null))
  (`/Engine/EditorBlueprintResources/StandardMacros.DoOnce` false :!label _label
    (:`Completed`
      (if (> (`self.requiredNpcCount`) (`self.SpawnedNpcCount`)) :!label _label_2
        (bind _npc (message `/Game/PedestrianSystem/Blueprints/BPI_NPCManagement.GetAvailableNPC` (`GameplayStatics.GetGameState`)))
        (`/Engine/EditorBlueprintResources/StandardMacros.IsValid` _npc
          (:`Is Valid`
            (set `self.Npc` _npc)
            (`self.K2_SetActorLocation` (`self.Npc`) _randomlocation false false)
            (`self.SetActorHiddenInGame` (`self.Npc`) false)
            (`KismetSystemLibrary.PrintString` "Taking available npc"))
          (:`Is Not Valid`
            (bind _returnvalue (`|SpawnActorFromClass` "/Game/PedestrianSystem/Blueprints/BP_Pedestrian.BP_Pedestrian_C" (`KismetMathLibrary.MakeTransform` _randomlocation (`KismetMathLibrary.MakeRotator` 0.0 0.0 (`KismetMathLibrary.RandomFloatInRange` 0.0 360.0))) "AdjustIfPossibleButDontSpawnIfColliding" "OverrideRootScale" null null))
            (`/Engine/EditorBlueprintResources/StandardMacros.IsValid` _returnvalue
              (:`Is Valid`
                (`KismetSystemLibrary.PrintString` "NPC Spawned" true true (struct :`R` 1.0 :`B` 0.027019 :`A` 1.0) 10.0)
                (set `self.Npc` _returnvalue))
              (:`Is Not Valid`
                (`KismetSystemLibrary.PrintString` "NPC  not Spawned" true true (struct :`G` 1.0 :`B` 0.064001 :`A` 1.0) 10.0)
                (`KismetSystemLibrary.Delay` 0.5)
                (goto _label_2)))))
        (`KismetArrayLibrary.Array_Add` (`self.SpawnedNPC`) (`self.Npc`))
        (`/Engine/EditorBlueprintResources/StandardMacros.IncrementInt` (`self.SpawnedNpcCount`)
          (:`  `
            (`KismetSystemLibrary.Delay` 0.2)
            (`Pawn.SpawnDefaultController` (`self.Npc`))
            (goto _label_2)))
        (else
          (goto _label :!via `Reset`))))))

(fn `CheckNPCLocation`
  (bind _spawnednpc (`self.SpawnedNPC`))
  (for _array_element _spawnednpc
    (if (> (`KismetMathLibrary.Vector_Distance` (`self.K2_GetActorLocation` (`self.PlayerRef`)) (`self.K2_GetActorLocation` _array_element)) (`self.NPCRange`))
      (message `/Game/PedestrianSystem/Blueprints/BPI_NPCManagement.AddAvailableNPC` (`GameplayStatics.GetGameState`) _array_element)
      (`self.SetActorHiddenInGame` _array_element true)
      (`KismetArrayLibrary.Array_RemoveItem` _spawnednpc _array_element)
      (`KismetSystemLibrary.PrintString` "Npc removed")
      (`/Engine/EditorBlueprintResources/StandardMacros.DecrementInt` (`self.SpawnedNpcCount`)))))

(fn `UserConstructionScript`)