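; BP_PointManager is a pedestrian system actor that populates a spline with NPC_Point actors when play begins.
; SpawnNPCPoints steps along the spline at PointSpacing intervals, spawning a point at each world-space location and storing it in NPCPointArray.
; Before spawning, it sets each stored point's lifespan to zero, which does not destroy the actor, and clears the array.
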(event `self.ReceiveBeginPlay`
  (`self.SpawnNPCPoints`))

(event `SpawnNPCPoints`
  (set `self.Distance` 0.0)
  (for _array_element (`self.NPC_PointArray`)
    (`self.SetLifeSpan` _array_element 0.0))
  (`KismetArrayLibrary.Array_Clear` (`self.NPC_PointArray`))
  (bind _returnvalue (`|SpawnActorFromClass` "/Game/PedestrianSystem/Blueprints/NPC_Point.NPC_Point_C" (`KismetMathLibrary.MakeTransform` (`SplineComponent.GetLocationAtDistanceAlongSpline` (`self.Spline`) (`self.Distance`) "World")) "Undefined" "OverrideRootScale" null null :!label _label))
  (bind _output_get (set `self.NPC_Point` _returnvalue))
  (`KismetArrayLibrary.Array_Add` (`self.NPC_PointArray`) _output_get)
  (set `self.Distance` (+ (`self.Distance`) (`self.PointSpacing`)))
  (if (< (`self.Distance`) (`SplineComponent.GetSplineLength` (`self.Spline`)))
    (goto _label)))

(fn `UserConstructionScript`)